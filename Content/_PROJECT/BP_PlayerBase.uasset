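; Player base actor that loses health when units from an opposing team reach it.
; When its Box component begins overlapping a BP_Unit with a different Team, it destroys that unit, subtracts a point of Health and prints the new value.
; Same-team units and other actors are ignored, and nothing here handles Health reaching zero.
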(event OnComponentBeginOverlap(Box)
  (params (OverlappedComponent :type Primitive%20Component%20Object%20Reference) (OtherActor :type Actor%20Object%20Reference) (OtherComp :type Primitive%20Component%20Object%20Reference) (OtherBodyIndex :type Integer) (bFromSweep :type Boolean) (SweepResult :type Hit%20Result%20Structure%20%28by%20ref%29))
  (bind _asbp_unit (Utilities|Casting|CastToBP_Unit OtherActor))
  (if (Utilities|Enum|NotEqual(Enum) (Variables|/Game/_PROJECT/BP_Unit.BP_Unit_C|GetTeam _asbp_unit) (Variables|Default|GetTeam))
    (Actor|DestroyActor _asbp_unit)
    (bind _output_get (Variables|Default|SetHealth (- (Variables|Default|GetHealth) 1.0)))
    (Development|PrintString (Utilities|String|Append "New health: " (Utilities|String|ToString(Float) _output_get)))))

(event EventBeginPlay)

(event Collision|EventActorBeginOverlap
  (params (OtherActor :type Actor%20Object%20Reference)))

(fn ConstructionScript)