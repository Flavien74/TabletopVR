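; Game mode that hosts and joins LAN multiplayer sessions through Advanced Sessions nodes.
; SearchSession runs a Gate-controlled loop that finds one session with a free slot and joins it, retrying on the next tick when the search or join fails.
; StopSearch, also called after a successful join, closes the gate and cancels searching.
; CreateSession creates a one-public-connection session and opens GameMap as a listen server.
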(event Custom|Create%20Session
  (|AdvancedSession 0 (Game|GetPlayerController 0) 1 0 true false false true true false false false true false true
    (:OnSuccess
      (Game|OpenLevel(byObjectReference) "/Game/_PROJECT/GameMap.GameMap" true "?listen"))))

(event Custom|Search%20Session
  (Utilities|FlowControl|Sequence
    (:then_0
      (goto _label Open))
    (:then_1
      (Utilities|FlowControl|Gate true :!label _label
        (:Exit
          (bind _results (|FindSessionsAdvanced 0 1 true "AllServers" 0 false false false 1)
            (:OnSuccess
              (if (Utilities|Array|IsEmpty _results)
                (CallFunction|ContinueSearch :!label _label_2)
                (else
                  (|JoinSession (Game|GetPlayerController 0) (Utilities|Array|Get(acopy) _results)
                    (:OnSuccess
                      (CallFunction|StopSearch))
                    (:OnFailure
                      (goto _label_2))))))
            (:OnFailure
              (CallFunction|ContinueSearch))))))))

(event Custom|Stop%20Search
  (Utilities|FlowControl|Sequence
    (:then_0
      (Utilities|FlowControl|Gate true) ; enters at Close
    )
    (:then_1
      (|CancelFindSessions (Game|GetPlayerController 0)))))

(event Custom|Continue%20Search
  (Utilities|FlowControl|DelayUntilNextTick)
  (Utilities|FlowControl|Gate true
    (:Exit
      (bind _results (|FindSessionsAdvanced 0 1 true "AllServers" 0 false false false 1)
        (:OnSuccess
          (if (Utilities|Array|IsEmpty _results)
            (CallFunction|ContinueSearch :!label _label)
            (else
              (|JoinSession (Game|GetPlayerController 0) (Utilities|Array|Get(acopy) _results)
                (:OnSuccess
                  (CallFunction|StopSearch))
                (:OnFailure
                  (goto _label))))))
        (:OnFailure
          (CallFunction|ContinueSearch))))))

(fn ConstructionScript)