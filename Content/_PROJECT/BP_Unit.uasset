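; BP_Unit is an auto-battler style combat unit that marches forward and fights units of other teams.
; Its Range sphere tracks opposing units, halting movement while any are inside and resuming once empty.
; A looping one-second timer damages the first tracked target, while point, radial and direct damage reduce health until the unit is destroyed.
; Each tick also draws the range sphere, colored by whether targets are present.
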(event OnComponentBeginOverlap(Range)
  (params (OverlappedComponent :type Primitive%20Component%20Object%20Reference) (OtherActor :type Actor%20Object%20Reference) (OtherComp :type Primitive%20Component%20Object%20Reference) (OtherBodyIndex :type Integer) (bFromSweep :type Boolean) (SweepResult :type Hit%20Result%20Structure%20%28by%20ref%29))
  (bind _asbp_unit (Utilities|Casting|CastToBP_Unit OtherActor))
  (if (Utilities|Enum|NotEqual(Enum) (Variables|Default|GetTeam) (Variables|BP_Unit_C|GetTeam _asbp_unit))
    (Utilities|Array|AddUnique (Variables|Default|GetInRange) _asbp_unit)
    (Variables|Default|SetCurrentSpeed 0.0)))

(event OnComponentEndOverlap(Range)
  (params (OverlappedComponent :type Primitive%20Component%20Object%20Reference) (OtherActor :type Actor%20Object%20Reference) (OtherComp :type Primitive%20Component%20Object%20Reference) (OtherBodyIndex :type Integer))
  (bind _asbp_unit (Utilities|Casting|CastToBP_Unit OtherActor))
  (Utilities|Array|RemoveItem (Variables|Default|GetInRange) _asbp_unit)
  (if (Utilities|Array|IsEmpty (Variables|Default|GetInRange))
    (Variables|Default|SetCurrentSpeed (Variables|Default|GetSpeed))))

(event Custom|Take%20Damage
  (params (Damage :type Float%20%28double-precision%29))
  (bind _self self)
  (bind _returnvalue (Utilities|GetDisplayName _self))
  (if (<= (- (Variables|Default|GetCurrentHealthPoints) Damage) 0.0) ; is dead
    (Variables|Default|SetCurrentHealthPoints 0.0)
    (Actor|DestroyActor)
    (Development|PrintString (Utilities|String|Append _returnvalue " is dead"))
    (else
      (bind _output_get (Variables|Default|SetCurrentHealthPoints (- (Variables|Default|GetCurrentHealthPoints) Damage)))
      (Development|PrintString (Utilities|String|Append _returnvalue " HP = " (Utilities|String|ToString(Float) _output_get))))))

(event Custom|Attack
  (if (Utilities|Array|IsNotEmpty (Variables|Default|GetInRange))
    (CallFunction|TakeDamage (Utilities|Array|Get(acopy) (Variables|Default|GetInRange)) (Variables|Default|GetCurrentAttackDamage))))

(event EventTick
  (params (DeltaSeconds :type Float%20%28single-precision%29))
  (Transformation|AddActorWorldOffset (* (* DeltaSeconds (Variables|Default|GetCurrentSpeed)) (Transformation|GetActorForwardVector)))
  (CallFunction|DrawDebug))

(event Game|Damage|EventPointDamage
  (params (Damage :type Float%20%28single-precision%29) (DamageType :type Damage%20Type%20Object%20Reference) (HitLocation :type Vector :default "0, 0, 0") (HitNormal :type Vector :default "0, 0, 0") (HitComponent :type Primitive%20Component%20Object%20Reference) (BoneName :type Name :default "None") (ShotFromDirection :type Vector :default "0, 0, 0") (InstigatedBy :type Controller%20Object%20Reference) (DamageCauser :type Actor%20Object%20Reference) (HitInfo :type Hit%20Result%20Structure%20%28by%20ref%29))
  (CallFunction|TakeDamage Damage))

(event Game|Damage|EventRadialDamage
  (params (DamageReceived :type Float%20%28single-precision%29) (DamageType :type Damage%20Type%20Object%20Reference) (Origin :type Vector :default "0, 0, 0") (HitInfo :type Hit%20Result%20Structure%20%28by%20ref%29) (InstigatedBy :type Controller%20Object%20Reference) (DamageCauser :type Actor%20Object%20Reference))
  (CallFunction|TakeDamage DamageReceived))

(event EventBeginPlay
  (Utilities|Time|SetTimerbyEvent (delegate Custom|Attack) 1.0 true false 0.0 1.0)
  (Variables|Default|SetCurrentAttackDamage (Variables|Default|GetAttackDamage))
  (Variables|Default|SetCurrentHealthPoints (Variables|Default|GetHealthPoints))
  (Variables|Default|SetCurrentSpeed (Variables|Default|GetSpeed)))

(fn ConstructionScript)

(fn DrawDebug
  (bind _range (Variables|Default|GetRange))
  (Rendering|Debug|DrawDebugSphere (Transformation|GetWorldLocation _range) (Class|SphereComponent|GetUnscaledSphereRadius _range) 12 (select (Utilities|Array|IsEmpty (Variables|Default|GetInRange)) "(R=0.000000,G=1.000000,B=0.002000,A=0.498000)" "(R=1.000000,G=0.000000,B=0.003000,A=0.499000)") 0.0))